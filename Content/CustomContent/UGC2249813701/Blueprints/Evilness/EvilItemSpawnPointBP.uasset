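; EvilItemSpawnPointBP is a spawn point that places a random item from AvailableItems at its transform.
; The game mode calls Reset on round starts, destroying any existing item and starting a new spawn cycle.
; SpawnItem waits a randomized delay, then spawns the item with an uncollected timeout.
; A half-second looping timer polls the item, restarting the cycle once it becomes invalid or is held by a player.
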(event `self.ReceiveBeginPlay`)

(event `SpawnItem`
  (bind _availableitems (`self.AvailableItems`))
  ;[1 1 1] Spawn Item (called via Reset() from Game-mode)
  (`KismetSystemLibrary.Delay` (+ (`self.MinSpawnDelay`) (`KismetMathLibrary.RandomFloatInRange` 0.0 (`self.SpawnDeviation`))))
  (bind _returnvalue (`|SpawnActorFromClass` (`|GetArrayItem` _availableitems (`KismetMathLibrary.RandomInteger` (`KismetArrayLibrary.Array_Length` _availableitems))) (`self.GetTransform`) "AlwaysSpawn" "OverrideRootScale" self (`self.DurationToShowFor`) null null))
  (set `self.SpawnedItem` _returnvalue)
  (bind _returnvalue_2 (`KismetSystemLibrary.K2_SetTimerDelegate` (delegate `CustomEvent_0`) 0.5 true))
  (set `self.TimerHandle` _returnvalue_2))

(event `CustomEvent_0`
  ;[1 1 1] Spawn Item (called via Reset() from Game-mode)
  (if (not (and (`KismetSystemLibrary.IsValid` (`self.SpawnedItem`)) (not (`/Game/CustomContent/UGC2249813701/Blueprints/Evilness/BaseEvilItemBP.HeldByPlayer` (`self.SpawnedItem`)))))
    (`KismetSystemLibrary.K2_ClearAndInvalidateTimerHandle` (`self.TimerHandle`))
    (`self.SpawnItem`)))

(event `Reset`
  ;[1 1 1] RESET (called from GM on round starts)  - Delete any old actor, spawn a new one
  (if (`KismetSystemLibrary.IsValid` (`self.SpawnedItem`))
    (`self.K2_DestroyActor` (`self.SpawnedItem`)))
  (set `self.SpawnedItem` null)
  ;[1 1 1] Reset logic
  (`KismetSystemLibrary.K2_ClearAndInvalidateTimerHandle` (`self.TimerHandle`))
  (`self.SpawnItem`))

(fn `UserConstructionScript`)