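; Base pickup item for the KJModEG game mode that players can pick up, drop or throw.
; On the server it finds the game-mode proxy, resolves overlapping pawns to player proxies and marks itself held if they can accept it.
; DroppedOrUsed detaches it, then either launches it along the player's forward vector with physics or uses a downward trace to rest it above the ground.
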(event `self.ReceiveBeginPlay`
  ;[0.5463 1 0] BEGINPLAY - On server find the game-mode, we use that to talk to player proxies
  (`/Engine/EditorBlueprintResources/ActorMacros.Switch Has Authority`
    (:`Authority`
      (bind _outactors (`GameplayStatics.GetAllActorsOfClass` "/Game/CustomContent/UGC2249813701/Blueprints/Gamemode/KJModEG_GameModeProxy.KJModEG_GameModeProxy_C"))
      (if (!= (`KismetArrayLibrary.Array_Length` _outactors) 1)
        (`KJModProxy.PrintString_KJMod` null "[Error] Did not find a single game-mode when there should be one" true true (struct :`R` 1.0 :`B` 0.095176 :`A` 1.0) 60.0)
        (else
          (set `self.KJModEGGameModeProxy` (`|GetArrayItem` _outactors)))))))

(event `self.ReceiveActorBeginOverlap`
  (params (OtherActor :type "Actor Object Reference"))
  ;[0.1719 1 0] OVERLAP - Detect a pawn overlapping us, look up their player proxy and fire the event
  (`/Engine/EditorBlueprintResources/ActorMacros.Switch Has Authority`
    (:`Authority`
      (if (not (`self.HeldByPlayer`))
        (bind _aspawn (cast `Pawn` OtherActor))
        (bind _asplayer_controller (cast `PlayerController` (`Pawn.GetController` _aspawn)))
        (bind _returnvalue (`KJModGameModeProxy.FindPlayerProxy` (`self.KJModEGGameModeProxy`) _asplayer_controller))
        (`/Engine/EditorBlueprintResources/StandardMacros.IsValid` _returnvalue
          (:`Is Valid`
            (bind _askjmod_eg_player_proxy (cast `/Game/CustomContent/UGC2249813701/Blueprints/PlayerRepresentation/KJModEG_PlayerProxy` _returnvalue))
            (bind _yes (`/Game/CustomContent/UGC2249813701/Blueprints/PlayerRepresentation/KJModEG_PlayerProxy.CanPickUpItem` _askjmod_eg_player_proxy))
            (if _yes
              (`/Game/CustomContent/UGC2249813701/Blueprints/PlayerRepresentation/KJModEG_PlayerProxy.ItemPickedUpByPlayer` _askjmod_eg_player_proxy self)
              (set `self.HeldByPlayer` true))))))))

(event `ThrowItemServer`
  (params (Force :type "Vector Structure"))
  (bind _returnvalue (`self.GetComponentByClass` "/Script/Engine.PrimitiveComponent"))
  ;[1 1 1] Throw Item (if supported)
  (`PrimitiveComponent.SetCollisionProfileName` _returnvalue "BlockAll" true)
  (`PrimitiveComponent.SetSimulatePhysics` _returnvalue true)
  (`PrimitiveComponent.AddForce` _returnvalue Force "None" true))

(fn `DroppedOrUsed`
  (params (OwningPlayerProxy :type "/Game/CustomContent/UGC2249813701/Blueprints/PlayerRepresentation/KJModEG_PlayerProxy Object Reference") (Throw :type Boolean))
  ;[1 1 1] Drop and detacth
  (`self.K2_DetachFromActor` self "KeepWorld" "KeepWorld" "KeepWorld")
  (if Throw
    ;[1 1 1] Throw with force
    (`self.ThrowItemServer` (* (`self.GetActorForwardVector` (`KJModPlayerProxy.playerPawn` OwningPlayerProxy)) 30000.0))
    (else
      ;[1 1 1] Ensure it sits on the ground
      (bind (_outhit _returnvalue) (`KismetSystemLibrary.LineTraceSingleForObjects` (`self.K2_GetActorLocation`) (- (`self.K2_GetActorLocation`) (0.0 0.0 1000.0)) (`|MakeArray` "ObjectTypeQuery1" "ObjectTypeQuery2" :!type "EObjectTypeQuery Enum")))
      (`self.K2_SetActorLocation` self (select `bool` _returnvalue :`false` (- (`self.K2_GetActorLocation`) (0.0 0.0 -125.0)) :`true` (+ (`.Location` (`GameplayStatics.BreakHitResult` _outhit)) (0.0 0.0 126.0))) false true))))

(fn `UserConstructionScript`)