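; Droppable item that, after a short pulsing fuse, becomes a stationary water tornado that grabs nearby characters, then destroys itself.
; Clients play the scale pulse, then hide the mesh and spawn the particle at a downward trace hit.
; The server enables the overlap sphere, switches entering characters to zero-gravity capsule physics, and pulls them toward the focal point each tick.
; Exit or expiry restores movement; the path-following logic is never run.
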(event `BombDroppedServer`
  (params (OwningPawnToIgnore :type "Pawn Object Reference"))
  ;[1 1 1] BOMB DROPPED SERVER - The bomb has been dropped by a player (via DroppedOrUsed function, inherited from the base item)
  (`self.BombDroppedClients`) ; Play visuals on the clients
  (`KismetSystemLibrary.Delay` 3.0) ; We're a 2 second "fuse"
  (`PrimitiveComponent.SetCollisionProfileName` (`self.SphereCollider`) "OverlapOnlyPawn" true)
  (`PrimitiveComponent.SetSimulatePhysics` (`self.StaticMesh`) false)
  (set `self.Activated` true)
  (`|ExecutionSequence`
    (:`then_0`
      (`KismetSystemLibrary.Delay` 10.0)
      (set `self.Activated` false)
      (`PrimitiveComponent.SetCollisionProfileName` (`self.SphereCollider`) "NoCollision" true)
      (for _array_element (`self.GrabbedCharacters`)
        (`self.SetPlayerPhysicsEnabledServer` false _array_element))
      (`KismetSystemLibrary.Delay` 1.0)
      (`self.K2_DestroyActor`))))

(event `self.ReceiveTick`
  (params (DeltaSeconds :type "Float (single-precision)"))
  (bind _returnvalue (`SceneComponent.K2_GetComponentLocation` (`self.FocalPoint`)))
  ;[1 1 1] EVENT TICK - Rotate the actor
  (if (`self.Activated`)
    (`|ExecutionSequence`
      (:`then_0`
        (`/Engine/EditorBlueprintResources/ActorMacros.Switch Has Authority`
          (:`Authority`
            ;[1 1 1] Pull all caught actors towards us
            (for _array_element (`PrimitiveComponent.GetOverlappingActors` (`self.SphereCollider`) null)
              (bind _ascharacter (cast `Character` _array_element))
              (bind _returnvalue_2 (`self.K2_GetActorLocation` _array_element))
              (`PrimitiveComponent.AddForce` (`Character.CapsuleComponent` _ascharacter) (* (* (`KismetMathLibrary.Conv_RotatorToVector` (`KismetMathLibrary.FindLookAtRotation` _returnvalue_2 _returnvalue)) (`KismetMathLibrary.VSize` (- _returnvalue _returnvalue_2))) 5.0) "None" true))))))
    (else
      (`self.K2_AddActorWorldRotation` (`KismetMathLibrary.MakeRotator` 0.0 0.0 (* DeltaSeconds 250.0))))))

(event `BombDroppedClients`
  (bind _returnvalue (`SceneComponent.K2_GetComponentLocation` (`self.StaticMesh`)))
  ;[1 1 1] BOMB DROPPED CLIENTS - Run visual pulsing of bomb before it explodes (and do explosion particles)
  (bind (_direction _scale) (`Timeline|Timeline_0` :!via `PlayFromStart`)
    (:`Update`
      (`SceneComponent.SetWorldScale3D` (`self.StaticMesh`) (`KismetMathLibrary.Conv_DoubleToVector` _scale)))
    (:`Finished`
      (`SceneComponent.SetWorldScale3D` (`self.StaticMesh`) (0.8 0.8 0.8))
      (`SceneComponent.SetVisibility` (`self.StaticMesh`) false false)
      (bind (_outhit _returnvalue_2) (`KismetSystemLibrary.LineTraceSingleForObjects` _returnvalue (- _returnvalue (0.0 0.0 1000.0)) (`|MakeArray` "ObjectTypeQuery1" "ObjectTypeQuery2" :!type "EObjectTypeQuery Enum")))
      (`GameplayStatics.SpawnEmitterAttached` "/Game/CustomContent/UGC2249813701/Particles/Particles/P_WaterTonardo.P_WaterTonardo" (`self.DefaultSceneRoot`) "None" (select `bool` _returnvalue_2 :`false` (`SceneComponent.K2_GetComponentLocation` (`self.StaticMesh`)) :`true` (`.Location` (`GameplayStatics.BreakHitResult` _outhit))) (struct) (2.5 2.5 2.5) "KeepWorldPosition"))))

(event `self.SphereCollider.OnComponentBeginOverlap`
  (params (OverlappedComponent :type "PrimitiveComponent Object Reference") (OtherActor :type "Actor Object Reference") (OtherComp :type "PrimitiveComponent Object Reference") (OtherBodyIndex :type Integer) (bFromSweep :type Boolean) (SweepResult :type "HitResult Structure (by ref)"))
  ;[1 1 1] Any characters near us? enable physics
  (`/Engine/EditorBlueprintResources/ActorMacros.Switch Has Authority`
    (:`Authority`
      (bind _ascharacter (cast `Character` OtherActor))
      (`self.SetPlayerPhysicsEnabledServer` true _ascharacter)
      (`KismetArrayLibrary.Array_Add` (`self.GrabbedCharacters`) _ascharacter))))

(event `self.SphereCollider.OnComponentEndOverlap`
  (params (OverlappedComponent :type "PrimitiveComponent Object Reference") (OtherActor :type "Actor Object Reference") (OtherComp :type "PrimitiveComponent Object Reference") (OtherBodyIndex :type Integer))
  ;[1 1 1] End overlap
  (`/Engine/EditorBlueprintResources/ActorMacros.Switch Has Authority`
    (:`Authority`
      (bind _ascharacter (cast `Character` OtherActor))
      (`self.SetPlayerPhysicsEnabledServer` false _ascharacter)
      (`KismetArrayLibrary.Array_RemoveItem` (`self.GrabbedCharacters`) _ascharacter))))

(event `SetPlayerPhysicsEnabledServer`
  (params (Disabled :type Boolean) (PlayerCharacter :type "Character Object Reference"))
  (bind _capsulecomponent (`Character.CapsuleComponent` PlayerCharacter))
  ;[1 1 1] Physics enable/disable
  (`self.SetPlayerPhysicsEnabledOwningClient` Disabled PlayerCharacter)
  (set `CharacterMovementComponent.GravityScale` (select `bool` Disabled :`false` 1.0 :!type "Float (single-precision)") (`self.GetComponentByClass` PlayerCharacter "/Script/Engine.CharacterMovementComponent"))
  (`PrimitiveComponent.SetSimulatePhysics` _capsulecomponent Disabled)
  (if (not Disabled)
    (`SceneComponent.K2_SetWorldRotation` :`self` _capsulecomponent :`bTeleport` true)))

(event `SetPlayerPhysicsEnabledOwningClient`
  (params (Disabled :type Boolean) (LocalPlayerCharacter :type "Character Object Reference"))
  (bind _capsulecomponent (`Character.CapsuleComponent` LocalPlayerCharacter))
  ;[1 1 1] Physics enable/disable
  (set `CharacterMovementComponent.GravityScale` (select `bool` Disabled :`false` 1.0 :!type "Float (single-precision)") (`self.GetComponentByClass` LocalPlayerCharacter "/Script/Engine.CharacterMovementComponent"))
  (`PrimitiveComponent.SetSimulatePhysics` _capsulecomponent Disabled)
  (if (not Disabled)
    (`SceneComponent.K2_SetWorldRotation` :`self` _capsulecomponent :`bTeleport` true)))

(fn `DroppedOrUsed`
  (params (OwningPlayerProxy :type "/Game/CustomContent/UGC2249813701/Blueprints/PlayerRepresentation/KJModEG_PlayerProxy Object Reference") (Throw :type Boolean))
  (`parent.DroppedOrUsed` OwningPlayerProxy false) ; Drop the item
  (`self.BombDroppedServer` null))

(fn `UserConstructionScript`
  (`parent.UserConstructionScript`))