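; Spinning bomb item, derived from a base item, that launches nearby characters upward when dropped or used, with no damage applied.
; DroppedOrUsed calls the parent, then a server event that triggers client visuals: a timeline pulses the mesh scale and spawns explosion particles when finished.
; After a two-second fuse, the server event sphere-overlaps pawns and launches characters vertically, harder the closer they are to the bomb.
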(event `self.ReceiveTick`
  (params (DeltaSeconds :type "Float (single-precision)"))
  ;[1 1 1] EVENT TICK - Rotate the actor
  (`self.K2_AddActorWorldRotation` (`KismetMathLibrary.MakeRotator` 0.0 0.0 (* DeltaSeconds 100.0))))

(event `BombDroppedServer`
  (params (OwningPawnToIgnore :type "Pawn Object Reference"))
  ;[1 1 1] BOMB DROPPED SERVER - The bomb has been dropped by a player (via DroppedOrUsed function, inherited from the base item)
  (`self.BombDroppedClients`) ; Play visuals on the clients
  (`KismetSystemLibrary.Delay` 2.0) ; We're a 2 second "fuse"
  (`KismetArrayLibrary.Array_Clear` (`self.FrozenPlayers`))
  (bind _outactors (`KismetSystemLibrary.SphereOverlapActors` (`SceneComponent.K2_GetComponentLocation` (`self.StaticMesh`)) 500.0 (`|MakeArray` "ObjectTypeQuery3" :!type "EObjectTypeQuery Enum") null (`|MakeArray` OwningPawnToIgnore :!type "Actor Object Reference"))) ; Get all pawn's in our blast window
  (for _array_element _outactors
    (bind _ascharacter (cast `Character` _array_element))
    (`Character.LaunchCharacter` _ascharacter (`KismetMathLibrary.MakeVector` 0.0 0.0 (* (- 500.0 (`KismetMathLibrary.Vector_Distance` (`self.K2_GetActorLocation` _ascharacter) (`SceneComponent.K2_GetComponentLocation` (`self.StaticMesh`)))) 3.0)) true true) ; Depending on distance from center, launch upwards
  ))

(event `BombDroppedClients`
  ;[1 1 1] BOMB DROPPED CLIENTS - Run visual pulsing of bomb before it explodes (and do explosion particles)
  (bind (_direction _scale) (`Timeline|Timeline_0` :!via `PlayFromStart`)
    (:`Update`
      (`SceneComponent.SetWorldScale3D` (`self.StaticMesh`) (`KismetMathLibrary.Conv_DoubleToVector` _scale)))
    (:`Finished`
      (`GameplayStatics.SpawnEmitterAtLocation` "/Game/CustomContent/UGC2249813701/Particles/Particles/P_Explosion.P_Explosion" (`SceneComponent.K2_GetComponentLocation` (`self.StaticMesh`))))))

(fn `DroppedOrUsed`
  (params (OwningPlayerProxy :type "/Game/CustomContent/UGC2249813701/Blueprints/PlayerRepresentation/KJModEG_PlayerProxy Object Reference") (Throw :type Boolean))
  (`parent.DroppedOrUsed` OwningPlayerProxy Throw) ; Drop the item
  (`self.BombDroppedServer` null))

(fn `UserConstructionScript`
  (`parent.UserConstructionScript`))