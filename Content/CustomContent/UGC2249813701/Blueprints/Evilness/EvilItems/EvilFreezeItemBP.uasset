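; Spinning freeze-bomb item that, once dropped or used, briefly freezes players caught within its blast radius.
; DroppedOrUsed starts the server event, which triggers client visuals (scale-pulse timeline, then ground-traced ice particles) and waits out a short fuse.
; A pawn sphere overlap is matched to player proxies, which are frozen, released after a delay, and then the item destroys itself.
; The owner-ignore input is left unset, so the dropper is not excluded.
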(event `self.ReceiveTick`
  (params (DeltaSeconds :type "Float (single-precision)"))
  (bind _returnvalue (* DeltaSeconds 125.0))
  ;[1 1 1] EVENT TICK - Rotate the actor
  (`self.K2_AddActorWorldRotation` (`KismetMathLibrary.MakeRotator` _returnvalue 0.0 _returnvalue)))

(event `BombDroppedServer`
  (params (OwningPawnToIgnore :type "Pawn Object Reference"))
  ;[1 1 1] BOMB DROPPED SERVER - The bomb has been dropped by a player (via DroppedOrUsed function, inherited from the base item)
  (`self.BombDroppedClients`) ; Play visuals on the clients
  (`KismetSystemLibrary.Delay` 2.0) ; We're a 2 second "fuse"
  (`KismetArrayLibrary.Array_Clear` (`self.FrozenPlayers`))
  (bind _outactors (`KismetSystemLibrary.SphereOverlapActors` (`SceneComponent.K2_GetComponentLocation` (`self.StaticMesh`)) 500.0 (`|MakeArray` "ObjectTypeQuery3" :!type "EObjectTypeQuery Enum") null (`|MakeArray` OwningPawnToIgnore :!type "Actor Object Reference"))) ; Get all pawn's in our blast window
  (for _array_element _outactors
    ;[1 1 1] Freeze all players for 2 seconds
    (bind _returnvalue (`KJModGameModeProxy.GetPlayerProxies` (`self.KJModEGGameModeProxy`)))
    (for _array_element_2 _returnvalue
      (if (== _array_element (`KJModPlayerProxy.playerPawn` _array_element_2))
        (bind _askjmod_eg_player_proxy (cast `/Game/CustomContent/UGC2249813701/Blueprints/PlayerRepresentation/KJModEG_PlayerProxy` _array_element_2))
        (`KismetArrayLibrary.Array_Add` (`self.FrozenPlayers`) _askjmod_eg_player_proxy)
        (break))))
  (`self.FreezePlayers`) ; After we're done, freeze those playes in place
)

(event `FreezePlayers`
  ;[1 1 1] FREEZE PLAYERS
  (for _array_element (`self.FrozenPlayers`)
    (`/Game/CustomContent/UGC2249813701/Blueprints/PlayerRepresentation/KJModEG_PlayerProxy.FreezePlayer` _array_element true))
  (`KismetSystemLibrary.Delay` 3.0) ; 3 seconds..
  (for _array_element_2 (`self.FrozenPlayers`)
    (`/Game/CustomContent/UGC2249813701/Blueprints/PlayerRepresentation/KJModEG_PlayerProxy.FreezePlayer` _array_element_2 false))
  (`KismetSystemLibrary.Delay` 3.0)
  (`self.K2_DestroyActor`))

(event `BombDroppedClients`
  (bind _returnvalue (`SceneComponent.K2_GetComponentLocation` (`self.StaticMesh`)))
  ;[1 1 1] BOMB DROPPED CLIENTS - Run visual pulsing of bomb before it explodes (and do explosion particles)
  (bind (_direction _scale) (`Timeline|Timeline_0` :!via `PlayFromStart`)
    (:`Update`
      (`SceneComponent.SetWorldScale3D` (`self.StaticMesh`) (`KismetMathLibrary.Conv_DoubleToVector` _scale)))
    (:`Finished`
      (bind (_outhit _returnvalue_2) (`KismetSystemLibrary.LineTraceSingleForObjects` _returnvalue (- _returnvalue (0.0 0.0 1000.0)) (`|MakeArray` "ObjectTypeQuery1" "ObjectTypeQuery2" :!type "EObjectTypeQuery Enum")))
      (`GameplayStatics.SpawnEmitterAtLocation` "/Game/CustomContent/UGC2249813701/Particles/Particles/P_Ice_Land.P_Ice_Land" (select `bool` _returnvalue_2 :`false` (`SceneComponent.K2_GetComponentLocation` (`self.StaticMesh`)) :`true` (`.Location` (`GameplayStatics.BreakHitResult` _outhit))) (struct) (2.5 2.5 2.5)))))

(fn `DroppedOrUsed`
  (params (OwningPlayerProxy :type "/Game/CustomContent/UGC2249813701/Blueprints/PlayerRepresentation/KJModEG_PlayerProxy Object Reference") (Throw :type Boolean))
  (`parent.DroppedOrUsed` OwningPlayerProxy Throw) ; Drop the item
  (`self.BombDroppedServer` null))

(fn `UserConstructionScript`
  (`parent.UserConstructionScript`))