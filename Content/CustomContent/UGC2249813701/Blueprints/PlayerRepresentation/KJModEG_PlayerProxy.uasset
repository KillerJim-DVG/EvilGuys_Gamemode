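; Player proxy for the Evil Guys KJMod game mode, representing each player in a gun-free, third-person round-based game.
; Server registers character models, attaches the proxy to the pawn and handles picking up, throwing or dropping evil items.
; Local client picks a random model, configures camera, chat and HUD, runs an eased intro camera sweep, and relays round phases.
; Macros split server/client and local/remote logic, with camera-facing name and position labels.
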(event `self.Initialised`
  ;[1 1 1] EVENT INTIALIZED
  (`self.HandleClientServerLogic`
    (:`ServerLogic`
      ;;[1 0 0.03409] SERVER SIDE - This game-mode has no default tools or guns, and we need to register our character models server side
      (`|ExecutionSequence`
        (:`then_0`
          ;;;[1 1 1] No guns or tools in this mode (or do we every "give" any)
          (`self.SetDefaultToolAndGunSettings` (make `KJModPlayerProxyDefaultToolAndGunSetting` "NoToolsOrGuns")))
        (:`then_1`
          ;;;[1 0.8312 0.3811] Add 20 male models
          (for _index (range 1 26)
            (bind _returnvalue (`KismetStringLibrary.Right` (`KismetStringLibrary.Concat_StrStr` "0" (`KismetStringLibrary.Conv_IntToString` _index)) 2))
            (`self.RegisterCharacterModel` (make `KJModCharacterModelTableRow` "" (`KismetStringLibrary.Concat_StrStr` "EvilGuys_CharacterM" _returnvalue) null "" (`|MakeArray` (`KismetStringLibrary.Concat_StrStr` "/Game/CustomContent/UGC2249813701/Characters/Meshes/Characters/SK_Male" _returnvalue)) "" "" "/Game/CustomContent/UGC2249813701/Characters/AnimBP/male/EvilGuys_Male_AnimBP"))))
        (:`then_2`
          ;;;[1 0.8312 0.3811] Add 20 female models
          (for _index_2 (range 1 26)
            (bind _returnvalue_2 (`KismetStringLibrary.Right` (`KismetStringLibrary.Concat_StrStr` "0" (`KismetStringLibrary.Conv_IntToString` _index_2)) 2))
            (`self.RegisterCharacterModel` (make `KJModCharacterModelTableRow` "" (`KismetStringLibrary.Concat_StrStr` "EvilGuys_CharacterF" _returnvalue_2) null "" (`|MakeArray` (`KismetStringLibrary.Concat_StrStr` "/Game/CustomContent/UGC2249813701/Characters/Meshes/Characters/SK_Female" _returnvalue_2)) "" "" "/Game/CustomContent/UGC2249813701/Characters/AnimBP/female/EvilGuys_Female_AnimBP"))))))
    (:`ClientLogic`
      (`self.LocalOrRemote`
        (:`IsLocal`
          ;;[0.4283 1 0.4172] Client Initialisation
          (`self.SetViewModes` "ThirdPerson") ; EG's always shows in First Person, so as soon as we're created (before a pawn exists) set up the mode
          (`|ExecutionSequence`
            (:`then_0`
              ;;;[0.03776 1 0] Select random male or female mode
              (`self.SetCharacterModel` (`KismetStringLibrary.Concat_StrStr` "EvilGuys_Character" (select `bool` (`KismetMathLibrary.RandomBool`) :`false` "M" :`true` "F") (`KismetStringLibrary.Right` (`KismetStringLibrary.Concat_StrStr` "0" (`KismetStringLibrary.Conv_IntToString` (`KismetMathLibrary.RandomIntegerInRange` 1 25))) 2))))
            (:`then_1`
              ;;;[0 1 0.01166] Evil Guy's has no running, crouching, third person only with camera offset (behind player), etc.
              (`self.SetMovementScope` (make `KJModPlayerProxyMovementScope` 600.0 600.0 1.0 true false (`KismetMathLibrary.MakeTransform` (-240.0 0.0 400.0) (struct :`Pitch` -40.0)) false 30.0))
              (`self.SetPlayerFrozen` (`self.ShouldBeginFrozen`)))
            (:`then_2`
              ;;;[0.1166 1 0] We want full control over the camera fading (we black it out whilst moving camera to sweep the level)
              (`self.DisableAutomaticFades` true)
              (`PlayerCameraManager.SetManualCameraFade` (`GameplayStatics.GetPlayerCameraManager` 0) 1.0 (struct :`A` 1.0) false))
            (:`then_3`
              ;;;[0 1 0.04714] Create the local HUD the player will see
              (bind _returnvalue_3 (`|CreateWidget` "/Game/CustomContent/UGC2249813701/Blueprints/PlayerRepresentation/HUDs/KJModEG_LocalPlayerHUDWidgetBP.KJModEG_LocalPlayerHUDWidgetBP_C" (`GameplayStatics.GetPlayerController` 0)))
              (bind _output_get (set `self.LocalPlayerHUDWidgetBP` _returnvalue_3))
              (`UserWidget.AddToViewport` _output_get 0) ; Always visible, the widgets in the HUD are invisible by default
            )
            (:`then_4`
              ;;;[0.1899 1 0] Set up text and voice chat to be global
              (`self.SetChatSettings` (make `KJModPlayerProxyChatSettings` true true false 0 "" (struct :`R` 1.0 :`G` 1.0 :`B` 1.0 :`A` 1.0) (0.0 -175.0)))
              (`self.SetVoiceSettings` (make `KJModPlayerProxyVoiceSettings` true true true false 3600.0 true 1 "Test" (struct :`R` 0.009775 :`B` 0.291667 :`A` 1.0) (0.0 0.0) true)))
            (:`then_5`
              ;;;[0.09515 1 0] No equipment bar (no guns!)
              (`self.SetEquipmentBarVisible` false))
            (:`then_6`
              ;;;[0.04439 1 0] We want input events (left/mouse) to be received
              (`self.EnableInput` (`self.playerController`)))))))))

(event `self.PlayerSpawnedWithPawn`
  ;[1 1 1] SPAWNED WITH PAWN - The player has been spawned, and pawn has just beedn created in the world for it
  (`self.HandleClientServerLogic` ; On clients only
    (:`ServerLogic`
      ;;[1 1 1] On server attach "us" to the player, this is because we've got a PlayerMarket (arrow) that we want above the pawn
      (`self.K2_AttachToActor` (`self.playerPawn`) "None" "SnapToTarget" "SnapToTarget" "SnapToTarget") ; Terrorist marker, "radar", etc. need this proxy to be welded to the actual player pawn
      (`self.K2_SetActorRelativeTransform` (`KismetMathLibrary.MakeTransform` (0.0 0.0 0.0)) false true) ; Ensure it's centered (no offset)
    )
    (:`ClientLogic`
      (`self.LocalOrRemote` ; For the "local" users player proxy
        (:`IsLocal`
          (`|ExecutionSequence`
            (:`then_0`
              ;;[1 1 1] Variable inits
              (set `self.SweepInProgress` false)
              (`SceneComponent.SetVisibility` (`self.PlayerMarker`) true false) ; The marker is not seen on remote players, just "us"
            )
            (:`then_1`
              ;;[1 1 1] Find start/end sweep that may be in the level, we move the camera from start to end when the player spawns
              (bind _outactors (`GameplayStatics.GetAllActorsWithTag` "StartCameraSweep"))
              (if (> (`KismetArrayLibrary.Array_Length` _outactors) 0)
                (set `self.StartSweepTransform` (`self.GetTransform` (`|GetArrayItem` _outactors)))
                ;;;[1 0.6282 0] End location is the player's pawn; adding in the offset the 3rd person camera is moved to (via SetMovementScope in Initialisation above)
                (set `self.EndSweepTransform` (`KismetMathLibrary.MakeTransform` (+ (`self.K2_GetActorLocation` (`self.playerPawn`)) (-240.0 0.0 400.0)) (struct :`Pitch` -40.0)))
                (set `self.SweepInProgress` true)
                (else
                  (set `self.SweepInProgress` false) ; Disable flag (set true by default)
                  (`/Game/CustomContent/UGC2249813701/Blueprints/PlayerRepresentation/HUDs/KJModEG_LocalPlayerHUDWidgetBP.ShowMapInformation` (`self.LocalPlayerHUDWidgetBP`)) ; No sweep? just show info immediately
                )))
            (:`then_2`
              ;;[1 1 1] Start the camera sweep (if the level contains the two start/end actors to use)
              (if (`self.SweepInProgress`)
                (`self.AllowCameraControl` true)
                (`self.SetCameraTransform` (`self.StartSweepTransform`)))
              (`PlayerCameraManager.StartCameraFade` (`GameplayStatics.GetPlayerCameraManager` 0) 1.0 0.0 1.0 (struct :`A` 1.0) false true))
            (:`then_3`
              ;;[1 1 1] Flag sets
              (set `self.Init` true)
              (`self.SetOpenTeamMicrophone` true true))))
        (:`IsRemote`
          (`self.ShowRemotePlayerName`))))))

(event `SpectatorSpawnedOwningClient`
  ;[1 1 1] SPECTATOR SPAWNED
  (`PlayerCameraManager.StartCameraFade` :`self` (`GameplayStatics.GetPlayerCameraManager` 0) :`FromAlpha` 1.0 :`Duration` 3.0 :`bHoldWhenFinished` true))

(event `AddWinner`
  (params (PlayerName :type String) (Time :type "Float (double-precision)"))
  ;[1 1 1] Add Winner
  (`/Game/CustomContent/UGC2249813701/Blueprints/PlayerRepresentation/HUDs/KJModEG_LocalPlayerHUDWidgetBP.SetWinner` (`self.LocalPlayerHUDWidgetBP`) PlayerName Time))

(event `self.ReceiveTick`
  (params (DeltaSeconds :type "Float (single-precision)"))
  ;[1 1 1] EVENT TICK
  (`self.HandleClientServerLogic` ; These are client (visual) functions
    (:`ClientLogic`
      (`self.FaceLocalPlayersCamera`)
      (if (`self.SweepInProgress`)
        (`self.SweepCameraAtStart` DeltaSeconds)))))

(event `SetWinnerNotificationServer`
  (params (Title :type String) (Visible :type Boolean))
  ;[1 1 1] Set winner (from game-mode)
  (`self.SetWinnerNotifiationMulticast` Title Visible))

(event `RoundStart`
  (params (Duration :type "Float (double-precision)"))
  ;[1 1 1] ROUND START - Unfreeze player
  (`/Game/CustomContent/UGC2249813701/Blueprints/PlayerRepresentation/HUDs/KJModEG_LocalPlayerHUDWidgetBP.RoundStarted` (`self.LocalPlayerHUDWidgetBP`) Duration)
  (`self.SetPlayerFrozen` false))

(event `SetWinnerNotifiationMulticast`
  (params (Title :type String) (Visible :type Boolean))
  ;[1 1 1] Set winner (from game-mode)
  (`TextRenderComponent.K2_SetText` (`self.txtPosition`) (`KismetTextLibrary.Conv_StringToText` Title)) ; Show position above player
  (`SceneComponent.SetVisibility` (`self.txtPosition`) Visible false) ; Make visible
)

(event `FinalBellPhaseStarted`
  (params (Duration :type "Float (double-precision)"))
  ;[1 1 1] Final Bell Phase
  (`/Game/CustomContent/UGC2249813701/Blueprints/PlayerRepresentation/HUDs/KJModEG_LocalPlayerHUDWidgetBP.FinalBellPhaseStarted` (`self.LocalPlayerHUDWidgetBP`) Duration))

(event `RoundFinished`
  ;[1 1 1] Round Finished
  (`/Game/CustomContent/UGC2249813701/Blueprints/PlayerRepresentation/HUDs/KJModEG_LocalPlayerHUDWidgetBP.RoundFinished` (`self.LocalPlayerHUDWidgetBP`))
  (`self.SetPlayerFrozen` true)
  (`KismetSystemLibrary.Delay` 3.0) ; Wait a couple of seconds
  (`PlayerCameraManager.StartCameraFade` (`GameplayStatics.GetPlayerCameraManager` 0) 0.0 1.0 1.0 (struct :`A` 1.0) false true))

(event `RoundReset`
  ;[1 1 1] Round Reset
  (`/Game/CustomContent/UGC2249813701/Blueprints/PlayerRepresentation/HUDs/KJModEG_LocalPlayerHUDWidgetBP.RoundReset` (`self.LocalPlayerHUDWidgetBP`))
  (`self.SetWinnerNotificationServer` "") ; Remove (any) position
)

(event `SetMapInformation`
  (params (MapName :type String) (MapDescription :type String))
  ;[1 1 1] SET MAP INFORMATION (game-mode sends us this event after spawning us)
  (`/Game/CustomContent/UGC2249813701/Blueprints/PlayerRepresentation/HUDs/KJModEG_LocalPlayerHUDWidgetBP.SetLevelInformation` (`self.LocalPlayerHUDWidgetBP`) MapName MapDescription))

(event `CountDownLockoutPhase`
  ;[1 1 1] Count down lock out, time to slide in UI
  (`/Game/CustomContent/UGC2249813701/Blueprints/PlayerRepresentation/HUDs/KJModEG_LocalPlayerHUDWidgetBP.CountDownLockoutPhase` (`self.LocalPlayerHUDWidgetBP`)))

(event `ItemPickedUpByPlayer`
  (params (Item :type "/Game/CustomContent/UGC2249813701/Blueprints/Evilness/BaseEvilItemBP Object Reference"))
  ;[1 1 1] ITEM PICKED UP - (Server) Called when a BaseEvilItem (that's not "held") overlaps THIS player
  (bind _output_get (set `self.HeldEvilItem` Item))
  ;;[1 1 1] On server attach "the" item to player, position above
  (`self.K2_AttachToActor` _output_get (`self.playerPawn`) "None" "SnapToTarget" "SnapToTarget" "SnapToTarget" true)
  (`self.K2_SetActorRelativeTransform` (`self.HeldEvilItem`) (`KismetMathLibrary.MakeTransform` (0.0 0.0 150.0) (struct) (0.5 0.5 0.5)) false true) ; Place above head
)

(event `Key|LeftMouseButton`
  (params (Key :type "Key Structure"))
  ;[1 1 1] LEFT MOUSE - Send event to server to throw the item
  (:`Pressed`
    (`self.ThrowEvilItemOwningClient`)))

(event `Key|RightMouseButton`
  (params (Key :type "Key Structure"))
  ;[1 1 1] RIGHT MOUSE - Drop
  (:`Pressed`
    (`self.DropEvilItemOwningClient`)))

(event `DropEvilItemOwningClient`
  ;[1 1 1] RIGHT MOUSE - Drop
  (`self.DropEvilItemServer`))

(event `ThrowEvilItemOwningClient`
  ;[1 1 1] LEFT MOUSE - Send event to server to throw the item
  (`self.ThrowEvilItemServer`))

(event `DropEvilItemServer`
  ;[1 1 1] DROP EVIL ITEM (Server) - Instruct the item to be evil
  (`/Engine/EditorBlueprintResources/StandardMacros.IsValid` (`self.HeldEvilItem`)
    (:`Is Valid`
      (`/Game/CustomContent/UGC2249813701/Blueprints/Evilness/BaseEvilItemBP.DroppedOrUsed` (`self.HeldEvilItem`) self false)
      (set `self.HeldEvilItem` null))))

(event `ThrowEvilItemServer`
  ;[1 1 1] THROW EVIL ITEM (Server) - Instruct the item to be evil
  (`/Engine/EditorBlueprintResources/StandardMacros.IsValid` (`self.HeldEvilItem`)
    (:`Is Valid`
      (`/Game/CustomContent/UGC2249813701/Blueprints/Evilness/BaseEvilItemBP.DroppedOrUsed` (`self.HeldEvilItem`) self true)
      (set `self.HeldEvilItem` null))))

(event `FreezePlayer`
  (params (Frozen :type Boolean))
  ;[1 1 1] Evil items can call this to freeze us; we're "owning client" as we can only run on clients (locally) and normally the server-side calls us
  (`self.SetPlayerFrozen` Frozen))

(fn `CameraSweepFinished`
  (bind _message (`self.Message`))
  ;[1 1 1] When the sweep is over, show any (ignored during sweep) message updates from the server
  (`/Game/CustomContent/UGC2249813701/Blueprints/PlayerRepresentation/HUDs/KJModEG_LocalPlayerHUDWidgetBP.ShowMessage` (`self.LocalPlayerHUDWidgetBP`) _message (not (`KismetStringLibrary.IsEmpty` _message)))
  ;[1 1 1] Allow player to move camera freely
  (`self.AllowCameraControl` false)
  (`/Game/CustomContent/UGC2249813701/Blueprints/PlayerRepresentation/HUDs/KJModEG_LocalPlayerHUDWidgetBP.ShowMapInformation` (`self.LocalPlayerHUDWidgetBP`)))

(fn `CanPickUpItem`
  (returns (Yes :type Boolean))
  (return (not (`KismetSystemLibrary.IsValid` (`self.HeldEvilItem`)))))

(fn `FaceLocalPlayersCamera`
  (`self.K2_SetActorRotation` (`KismetMathLibrary.FindLookAtRotation` (`KismetMathLibrary.MakeVector` (.x (`self.K2_GetActorLocation`)) (.y (`self.K2_GetActorLocation`))) (`KismetMathLibrary.MakeVector` (.x (`PlayerCameraManager.GetCameraLocation` (`GameplayStatics.GetPlayerCameraManager` 0))) (.y (`PlayerCameraManager.GetCameraLocation` (`GameplayStatics.GetPlayerCameraManager` 0))))) true) ; Rotate us to face the local camera (player)
)

(fn `OnRep_Message`
  (bind _message (`self.Message`))
  ;[1 1 1] If the game-mode set's a message on us, then display it
  (`self.LocalOrRemote`
    (:`IsLocal`
      (if (and (not (`self.SweepInProgress`)) (`self.Init`))
        (`/Game/CustomContent/UGC2249813701/Blueprints/PlayerRepresentation/HUDs/KJModEG_LocalPlayerHUDWidgetBP.ShowMessage` (`self.LocalPlayerHUDWidgetBP`) _message (not (`KismetStringLibrary.IsEmpty` _message)))))))

(fn `OnRep_ShouldBeginFrozen`
  (`self.SetPlayerFrozen` (`self.ShouldBeginFrozen`)))

(fn `PrintDebugMessage`
  (params (Message :type String) (Color :type "LinearColor Structure" :default (struct :`R` 1.0 :`G` 1.0 :`B` 1.0 :`A` 1.0)) (Duration :type "Float (double-precision)" :default 15.0))
  ;[1 1 1] We use the PrintString from KJMod as UE4 doesn't support "PrintString" at run-time in shipping games; we wrap it in a bool to enable/disable
  (if (`self.EnableDebugPrinting`)
    (`KJModProxy.PrintString_KJMod` null Message true true Color Duration)))

(fn `ShowRemotePlayerName`
  (`TextRenderComponent.K2_SetText` (`self.txtPlayerName`) (`KismetTextLibrary.Conv_StringToText` (`PlayerState.GetPlayerName` (`self.playerState`))))
  (`SceneComponent.SetVisibility` (`self.txtPlayerName`) true false))

(fn `SweepCameraAtStart`
  (params (Delta :type "Float (double-precision)"))
  ;[1 1 1] Accumulate time over 10 seconds (alpha 0..1)
  (bind _output_get (set `self.SweepProgress` (`KismetMathLibrary.FMin` (+ (/ Delta 10.0) (`self.SweepProgress`)) 1.0)))
  (bind _result (`|EaseFunction` "EaseInOut" _output_get 0.0 1.0))
  ;[1 1 1] Ease in/out camera movement over the 10 seconds
  (`self.SetCameraTransform` (`KismetMathLibrary.TLerp` (`self.StartSweepTransform`) (`self.EndSweepTransform`) _result))
  ;[1 1 1] Done? clear flag
  (if (>= _result 1.0)
    (set `self.SweepInProgress` false)
    ;[1 0.3142 0.08274] Do completion stuff
    (`self.CameraSweepFinished`)))

(fn `UserConstructionScript`)