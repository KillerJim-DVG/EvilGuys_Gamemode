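; Server-side game mode proxy for an Evil Guys mod: a round-based race to an end zone, with ranked finishers.
; A one-second timer drives a state machine from waiting and countdown through main phase, final bell (first finisher or last minute) and reset.
; It spawns a proxy per player to relay round events, messages and winners; late joiners spectate.
; Levels supply durations, map text and finish overlaps through events, plus tagged actors that become item spawners.
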(event `self.GameModeActivated`
  ;[1 0.8675 0.1036] GAME MODE ACTIVATED EVENT
  ;;[1 1 1] Always spawn our players as spectators initially, we will make them full players later
  (`self.SetJoiningPlayersParameters` (make `KJModGameModeProxyPlayerJoinParameters` true 0.0 false 5.0 0.0))
  (`self.SwitchToNewState` "NewEnumerator5"))

(event `self.ReceiveBeginPlay`
  ;[0.2965 1 0.1402] BEGIN PLAY - Process state machine every second
  (`self.InitialiseEvilSpawners`)
  (`KismetSystemLibrary.K2_SetTimerDelegate` (delegate `StateMachineEvent`) 1.0 true) ; Set up our 1 second timer to look after states
)

(event `StateMachineEvent`
  ;[0.2965 1 0.1402] BEGIN PLAY - Process state machine every second
  (switch `/Game/CustomContent/UGC2249813701/Blueprints/Gamemode/Enums/KJModEG_GameMode_Phase` (`self.State`)
    (:`NewEnumerator5`
      (`self.HandleGameReset`))
    (:`NewEnumerator1`
      (`self.Handle Waiting on Numbers`))
    (:`NewEnumerator2`
      (`self.HandleCountDown`))
    (:`NewEnumerator7`
      (`self.HandleCountDownLockOut`))
    (:`NewEnumerator3`
      (`self.HandleMainPhase`))
    (:`NewEnumerator8`
      (`self.HandleFinalBellPhase`))
    (:`NewEnumerator4`
      (`self.HandleEndPhase`))))

(event `PlayerReachedFinishedCollider`
  (params (PlayerController :type "PlayerController Object Reference"))
  (bind _coursecompletedplayers (`self.CourseCompletedPlayers`))
  (bind _returnvalue (`KismetArrayLibrary.Array_Length` _coursecompletedplayers))
  ;[1 0.4961 0.0398] PLAYER REACHED FINISH COLLIDER - An actor on the level has issued an event to us (via the SDK) showing a player has overlapped the end zone
  (for _array_element (`self.EGPlayerRepresentation`)
    (bind _playercontroller (`KJModPlayerProxy.playerController` _array_element))
    ;;[1 1 1] Was this player the one who hit the finish collider?
    (if (== PlayerController _playercontroller)
      ;;[1 1 1] Have they already finished?
      (if (< (`KismetArrayLibrary.Array_Find` (`self.CourseCompletedPlayers`) _array_element) 0)
        ;;[1 1 1] First winner? start final bell phase
        (if (`|EnumEquality` (`self.State`) "NewEnumerator3")
          (`self.SwitchToNewState` "NewEnumerator8"))
        ;;[1 1 1] Record this winner
        (`KismetArrayLibrary.Array_Add` _coursecompletedplayers _array_element)
        ;;[1 1 1] First 5 get positions above their heads
        (if (<= _returnvalue 5)
          (`/Game/CustomContent/UGC2249813701/Blueprints/PlayerRepresentation/KJModEG_PlayerProxy.SetWinnerNotificationServer` _array_element (select `int` _returnvalue :`0` "" :`1` "1st" :`2` "2nd" :`3` "3rd" :`4` "4th" :`5` "5th") true))
        ;;[1 1 1] Have all players finished? Is round over?
        (if (== (`KismetArrayLibrary.Array_Length` (`self.CourseCompletedPlayers`)) (`KismetArrayLibrary.Array_Length` (`self.EGPlayerRepresentation`)))
          (`self.SwitchToNewState` "NewEnumerator4"))
        ;;[1 1 1] Tell every proxy (including ourselves) about this winner, then break (finish)
        (for _array_element_2 (`self.EGPlayerRepresentation`)
          (`/Game/CustomContent/UGC2249813701/Blueprints/PlayerRepresentation/KJModEG_PlayerProxy.AddWinner` _array_element_2 (`AdvancedSessionsLibrary.GetPlayerName` _playercontroller) (`self.MainPhaseTimeout`)))
        (break)
        (else
          (break))))))

(event `self.EventFired_PlayerControllerParam`
  (params (EventName :type String) (playerController :type "PlayerController Object Reference"))
  ;[1 1 1] EVENT (From level, or other actors not part of the game-mode) - PLAYER CONTROLLER PARAM
  (switch `string` EventName
    (:`EndZoneOverlap`
      (`self.PlayerReachedFinishedCollider` playerController) ; A KJModEG_EndZone create this event when a player touches the finish collider
    )))

(event `self.EventFired_FloatParam`
  (params (EventName :type String) (value :type "Float (single-precision)"))
  ;[1 1 1] EVENT (From level, or other actors not part of the game-mode) - FLOAT PARAMS
  (switch `string` EventName
    (:`EvilGuysMapsTime`
      (set `self.LevelDuration` value) ; Level's can supply the game length
    )
    (:`EvilGuysFinalBellTime`
      (set `self.FinalBellDuration` value))))

(event `self.EventFired_StringParam`
  (params (EventName :type String) (value :type String))
  ;[1 1 1] EVENT (From level, or other actors not part of the game-mode) - STRING PARAMS
  (switch `string` EventName
    (:`EvilGuysMapName`
      (set `self.MapName` value))
    (:`EvilGuysMapDescription`
      (set `self.MapDescription` value))))

(fn `Check Enough Players`
  (if (< (`self.CurrentPlayerCount`) (`self.MinPlayers`))
    (`self.SwitchToNewState` "NewEnumerator5")))

(fn `Handle Waiting on Numbers`
  (if (>= (`self.CurrentPlayerCount`) (`self.MinPlayers`))
    ;[1 1 1] Enough players have arrived, move on
    (`self.SwitchToNewState` "NewEnumerator2")
    (`self.Show Information to All Players` "")
    (else
      ;[1 1 1] If waiting, show information to clients
      (`self.Show Information to All Players` (`KismetStringLibrary.Concat_StrStr` "Waiting on " (`KismetStringLibrary.Conv_IntToString` (`self.MinPlayers`)) " players to begin the game...") true))))

(fn `HandleCountDown`
  (bind _result (`/Engine/EditorBlueprintResources/StandardMacros.DecrementInt` (`self.CountDownTimeout`))
    (:`  `
      (if (<= _result 5)
        (`self.Show Information to All Players` "5" true) ; Hide
        (`self.SwitchToNewState` "NewEnumerator7")
        (else
          (`self.Show Information to All Players` (`KismetStringLibrary.Concat_StrStr` "Round starts in " (`KismetStringLibrary.Conv_IntToString` (`self.CountDownTimeout`)) "...") true))))))

(fn `HandleCountDownLockOut`
  (bind _result (`/Engine/EditorBlueprintResources/StandardMacros.DecrementInt` (`self.CountDownTimeout`))
    (:`  `
      (if (<= _result 0)
        (`self.Show Information to All Players` "") ; Hide
        (`self.SwitchToNewState` "NewEnumerator3")
        (else
          (`self.Show Information to All Players` (`KismetStringLibrary.Conv_IntToString` (`self.CountDownTimeout`)) true))))))

(fn `HandleEndPhase`
  (bind _result (`/Engine/EditorBlueprintResources/StandardMacros.DecrementFloat` (`self.EndPhaseTimeout`))
    (:`  `
      (if (< _result 1.0)
        (`self.SwitchToNewState` "NewEnumerator5")))))

(fn `HandleFinalBellPhase`
  (`/Engine/EditorBlueprintResources/StandardMacros.DecrementFloat` (`self.MainPhaseTimeout`)
    (:`  `
      (bind _result (`/Engine/EditorBlueprintResources/StandardMacros.DecrementFloat` (`self.FinalBellPhaseTimeout`))
        (:`  `
          (if (< _result 1.0)
            (`self.SwitchToNewState` "NewEnumerator4")))))))

(fn `HandleGameReset`
  (`self.PrintDebugMessage` "[Mod State] Game Reset Called" (struct :`R` 0.431641 :`G` 0.479585 :`B` 0.609375 :`A` 1.0))
  (`|ExecutionSequence`
    (:`then_0`
      (set `self.CountDownTimeout` (`self.CountDownDuration`)))
    (:`then_1`
      (set `self.EndPhaseTimeout` 5.0) ; Round end is always 5 seconds
    )
    (:`then_2`
      (`KismetArrayLibrary.Array_Clear` (`self.CourseCompletedPlayers`)) ; Forget about last winners
    )
    (:`then_3`
      (`self.SwitchToNewState` "NewEnumerator1"))))

(fn `HandleMainPhase`
  (bind _result (`/Engine/EditorBlueprintResources/StandardMacros.DecrementFloat` (`self.MainPhaseTimeout`)) ; Last 60 seconds is the "final bell phase" (unless a player has reached the end before that, in which case we're switched to final phase external to this function)
    (:`  `
      (if (< _result 61.0)
        (`self.SwitchToNewState` "NewEnumerator8")))))

(fn `InitialiseEvilSpawners`
  (bind _outactors (`GameplayStatics.GetAllActorsWithTag` "EvilSpawner"))
  (for _array_element _outactors
    (`|SpawnActorFromClass` "/Game/CustomContent/UGC2249813701/Blueprints/Evilness/EvilItemSpawnPointBP.EvilItemSpawnPointBP_C" (`self.GetTransform` _array_element) "AlwaysSpawn" "OverrideRootScale" self null)))

(fn `PlayerHasJoined`
  (params (joiningPlayerController :type "PlayerController Object Reference"))
  (returns (ReturnValue :type "KJModPlayerProxy Object Reference"))
  ;[1 1 1] SERVER - Handle player joining
  (set `self.CurrentPlayerCount` (+ (`self.CurrentPlayerCount`) 1))
  (`self.PrintDebugMessage` "[Mod] Player Has Joined" (struct :`R` 0.306297 :`G` 1.0 :`A` 1.0) 5.0)
  ;[1 1 1] Spawn the TTT player proxy (i.e. player representation)
  (bind _returnvalue (`|SpawnActorFromClass` "/Game/CustomContent/UGC2249813701/Blueprints/PlayerRepresentation/KJModEG_PlayerProxy.KJModEG_PlayerProxy_C" (`KismetMathLibrary.MakeTransform` (0.0 0.0 0.0)) "Undefined" "OverrideRootScale" joiningPlayerController null)) ; Note: As we run on server, we set owner of the player representation to the new controller (for "Execute On Owning Client" Events sent to it)
  ;[1 1 1] Record it, and initialise it with the related player controller
  (`KismetArrayLibrary.Array_Add` (`self.EGPlayerRepresentation`) _returnvalue) ; Record it, so we can destroy it later
  (`KJModPlayerProxy.Initialise` _returnvalue joiningPlayerController self (make `KJModPlayerProxyPawnSettings` 100 0 false true true)) ; Must call initialise after spawning, must include player controller
  ;[1 1 1] Tell the player about the map (received from level)
  (`/Game/CustomContent/UGC2249813701/Blueprints/PlayerRepresentation/KJModEG_PlayerProxy.SetMapInformation` _returnvalue (`self.MapName`) (`self.MapDescription`))
  ;[0.6744 1 0.9601] Has the player joined in a state where they should immediately spawn?
  (if (select `/Game/CustomContent/UGC2249813701/Blueprints/Gamemode/Enums/KJModEG_GameMode_Phase` (`self.State`) :`NewEnumerator5` true :`NewEnumerator1` true :`NewEnumerator2` true :`NewEnumerator7` true :`NewEnumerator3` true)
    (`self.SpawnPlayer` _returnvalue) ; Note: As we have set up this GM to have joining players as spectators this will take a full second FULL SECOND to spawn the real player pawn.
    ;[1 1 1] Handle players who appear in main game, allow them to move..
    (set `/Game/CustomContent/UGC2249813701/Blueprints/PlayerRepresentation/KJModEG_PlayerProxy.ShouldBeginFrozen` (select `/Game/CustomContent/UGC2249813701/Blueprints/Gamemode/Enums/KJModEG_GameMode_Phase` (`self.State`) :`NewEnumerator5` true :`NewEnumerator1` true :`NewEnumerator2` true :`NewEnumerator7` true) _returnvalue)
    (else
      ;[1 1 1] Handle Spectators
      (`/Game/CustomContent/UGC2249813701/Blueprints/PlayerRepresentation/KJModEG_PlayerProxy.SpectatorSpawnedOwningClient` _returnvalue) ; Spectator needs faded up to see the on-going game
    ))
  (return _returnvalue))

(fn `PlayerHasLeft`
  (params (leavingPlayerController :type "PlayerController Object Reference"))
  (returns (ReturnValue :type Boolean))
  ;[1 1 1] Reduce active player counts
  (set `self.CurrentPlayerCount` (- (`self.CurrentPlayerCount`) 1))
  (`self.PrintDebugMessage` "[Mod] Player Has left" (struct :`R` 0.786458 :`B` 0.062841 :`A` 1.0))
  ;[1 1 1] Search all previously recorded player representations for a matching entry
  (for _array_element (`self.EGPlayerRepresentation`)
    (if (== leavingPlayerController (`KJModPlayerProxy.playerController` _array_element))
      ;[1 1 1] Destroy and forget about it
      (`self.K2_DestroyActor` _array_element) ; Destroy it
      (`KismetArrayLibrary.Array_RemoveItem` (`self.EGPlayerRepresentation`) _array_element) ; Remove from array
      (return false) ; No errors
    ))
  (`self.PrintDebugMessage` "[Mod] Could not find the leaving player!!!!" (struct :`R` 0.786458 :`B` 0.062841 :`A` 1.0))
  (return true) ; Should never reach here!
)

(fn `PrintDebugMessage`
  (params (Message :type String) (Color :type "LinearColor Structure" :default (struct :`R` 1.0 :`G` 1.0 :`B` 1.0 :`A` 1.0)) (Duration :type "Float (double-precision)" :default 15.0))
  ;[1 1 1] We use the Print Debug Message in the Proxy, UE4 doesn't support "PrintString" at run-time in shipping games
  (if (`self.ShouldDebugPrintGameMode`)
    (`KJModProxy.PrintString_KJMod` null Message true true Color Duration)
    (`KismetSystemLibrary.PrintString` Message true true Color Duration)))

(fn `Show Information to All Players`
  (params (Message :type String) (ShowMessage :type Boolean))
  ;[1 1 1] Show a message to all remote players; used for showing like "waiting players", "get ready", etc.
  (bind _returnvalue (`self.GetPlayerProxies`))
  (for _array_element _returnvalue
    (bind _askjmod_eg_player_proxy (cast `/Game/CustomContent/UGC2249813701/Blueprints/PlayerRepresentation/KJModEG_PlayerProxy` _array_element))
    (set `/Game/CustomContent/UGC2249813701/Blueprints/PlayerRepresentation/KJModEG_PlayerProxy.Message` (select `bool` ShowMessage :`true` Message) _askjmod_eg_player_proxy)))

(fn `SwitchToNewState`
  (params (State :type "/Game/CustomContent/UGC2249813701/Blueprints/Gamemode/Enums/KJModEG_GameMode_Phase Enum" :default "NewEnumerator5"))
  ;[1 1 1] Called only when entering a "new" state, so performs one time only set-up for the new state
  (bind _output_get (set `self.State` State))
  (`self.PrintDebugMessage` (`KismetStringLibrary.Concat_StrStr` "[Mod] Switching to new state: " (`|GetEnumeratorNameAsString` _output_get)) (struct :`R` 0.601397 :`G` 0.567708 :`B` 1.0 :`A` 1.0))
  (switch `/Game/CustomContent/UGC2249813701/Blueprints/Gamemode/Enums/KJModEG_GameMode_Phase` State
    (:`NewEnumerator5`
      ;[1 1 1] Round Finished
      (for _array_element (`self.EGPlayerRepresentation`)
        (`/Game/CustomContent/UGC2249813701/Blueprints/PlayerRepresentation/KJModEG_PlayerProxy.RoundReset` _array_element)
        (`self.SpawnPlayer` _array_element)))
    (:`NewEnumerator7`
      ;[1 1 1] Tell clients we're about to start (they'll slide in UI elements, etc.)
      (for _array_element_2 (`self.EGPlayerRepresentation`)
        (`/Game/CustomContent/UGC2249813701/Blueprints/PlayerRepresentation/KJModEG_PlayerProxy.CountDownLockoutPhase` _array_element_2)))
    (:`NewEnumerator3`
      ;[1 1 1] Send a message to all players that the round has begun!
      (bind _output_get_2 (set `self.MainPhaseTimeout` (`self.LevelDuration`)))
      (for _array_element_3 (`self.EGPlayerRepresentation`)
        (`/Game/CustomContent/UGC2249813701/Blueprints/PlayerRepresentation/KJModEG_PlayerProxy.RoundStart` _array_element_3 _output_get_2)
        ;[1 1 1] Reset evil spawners
        (bind _outactors (`GameplayStatics.GetAllActorsOfClass` "/Game/CustomContent/UGC2249813701/Blueprints/Evilness/EvilItemSpawnPointBP.EvilItemSpawnPointBP_C"))
        (for _array_element_4 _outactors
          (`/Game/CustomContent/UGC2249813701/Blueprints/Evilness/EvilItemSpawnPointBP.Reset` _array_element_4))))
    (:`NewEnumerator8`
      ;[1 1 1] Send a message to all players that the round has begun!
      (bind _output_get_3 (set `self.FinalBellPhaseTimeout` (`self.FinalBellDuration`)))
      (for _array_element_5 (`self.EGPlayerRepresentation`)
        (`/Game/CustomContent/UGC2249813701/Blueprints/PlayerRepresentation/KJModEG_PlayerProxy.FinalBellPhaseStarted` _array_element_5 _output_get_3)))
    (:`NewEnumerator4`
      ;[1 1 1] Round Finished
      (for _array_element_6 (`self.EGPlayerRepresentation`)
        (`/Game/CustomContent/UGC2249813701/Blueprints/PlayerRepresentation/KJModEG_PlayerProxy.RoundFinished` _array_element_6)))))

(fn `UserConstructionScript`)